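; Enemy spawner actor that periodically spawns BP_EnemyCharacter AI at its own location.
; A looping timer started on BeginPlay counts all enemy characters in the level and spawns one only while that count is below MaxEnemies.
; SpawnEnemy uses SpawnAIFromClass with BT_EnemyBehavior; a random navigable-point lookup is present but unused.
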(event Custom|TryToSpawnEnemy
  (bind _outactors (Actor|GetAllActorsOfClass "/Game/Enemies/Enemy/BP_EnemyCharacter.BP_EnemyCharacter_C"))
  (if (< (Utilities|Array|Length _outactors) (Variables|Default|GetMaxEnemies))
    (Utilities|SpawnEnemy)))

(event EventBeginPlay
  (Utilities|Time|SetTimerbyEvent (delegate Custom|TryToSpawnEnemy) (Variables|Default|GetSpawnTime) true))

(event Collision|EventActorBeginOverlap
  (params (OtherActor :type Actor%20Object%20Reference)))

(event EventTick
  (params (DeltaSeconds :type Float%20%28single-precision%29)))

(fn ConstructionScript)