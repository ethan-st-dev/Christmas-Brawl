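; Enemy character for a VR shooter that patrols between two points and can be destroyed by player weapons.
; Overlapping either patrol point switches the target to the other and writes it to the blackboard; the initial patrol assignment is unconnected.
; ShotgunBlast overlaps and Projectile hits share one damage path that decrements health.
; At last health, it spawns an explosion, increments the VRPawn's TargetsEliminated count and destroys itself.
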(event OnComponentHit(CapsuleComponent)
  (params (HitComponent :type Primitive%20Component%20Object%20Reference) (OtherActor :type Actor%20Object%20Reference) (OtherComp :type Primitive%20Component%20Object%20Reference) (NormalImpulse :type Vector :default "0, 0, 0") (Hit :type Hit%20Result%20Structure%20%28by%20ref%29)))

(event OnComponentHit(Mesh)
  (params (HitComponent :type Primitive%20Component%20Object%20Reference) (OtherActor :type Actor%20Object%20Reference) (OtherComp :type Primitive%20Component%20Object%20Reference) (NormalImpulse :type Vector :default "0, 0, 0") (Hit :type Hit%20Result%20Structure%20%28by%20ref%29)))

(event Collision|EventActorBeginOverlap
  (params (OtherActor :type Actor%20Object%20Reference))
  (Utilities|Casting|CastToShotgunBlast OtherActor
    (:then
      (if (> (Variables|Default|GetEnemyHealth) 1)
        (Math|Integer|DecrementInt (Variables|Default|GetEnemyHealth))
        (else
          (Game|SpawnActorfromClass "/Game/StarterContent/Blueprints/Blueprint_Effect_Explosion.Blueprint_Effect_Explosion_C" (Transformation|GetActorTransform) "Undefined" 0 0)
          (bind _asvrpawn (Utilities|Casting|CastToVRPawn (Game|Player|GetPlayerPawn 0)))
          (Math|Integer|IncrementInt (Variables|/Game/VRTemplate/Blueprints/VRPawn.VRPawn_C|GetTargetsEliminated _asvrpawn)
            (:%20%20
              (Actor|DestroyActor))))))
    (:CastFailed
      (if (== (Variables|Default|GetPatrolPoint1) OtherActor)
        (Variables|Default|SetCurrentPatrolPoint (Variables|Default|GetPatrolPoint2))
        (Utilities|UpdatePatrolPointBB: :!label _label)
        (elif (== OtherActor (Variables|Default|GetPatrolPoint2))
          (Variables|Default|SetCurrentPatrolPoint (Variables|Default|GetPatrolPoint1))
          (goto _label))))))

(event EventTick
  (params (DeltaSeconds :type Float%20%28single-precision%29)))

(event Collision|EventHit
  (params (MyComp :type Primitive%20Component%20Object%20Reference) (Other :type Actor%20Object%20Reference) (OtherComp :type Primitive%20Component%20Object%20Reference) (bSelfMoved :type Boolean) (HitLocation :type Vector :default "0, 0, 0") (HitNormal :type Vector :default "0, 0, 0") (NormalImpulse :type Vector :default "0, 0, 0") (Hit :type Hit%20Result%20Structure%20%28by%20ref%29))
  (Utilities|Casting|CastToProjectile Other)
  (if (> (Variables|Default|GetEnemyHealth) 1)
    (Math|Integer|DecrementInt (Variables|Default|GetEnemyHealth))
    (else
      (Game|SpawnActorfromClass "/Game/StarterContent/Blueprints/Blueprint_Effect_Explosion.Blueprint_Effect_Explosion_C" (Transformation|GetActorTransform) "Undefined" 0 0)
      (bind _asvrpawn (Utilities|Casting|CastToVRPawn (Game|Player|GetPlayerPawn 0)))
      (Math|Integer|IncrementInt (Variables|/Game/VRTemplate/Blueprints/VRPawn.VRPawn_C|GetTargetsEliminated _asvrpawn)
        (:%20%20
          (Actor|DestroyActor))))))

(fn ConstructionScript
  (|CallParentFunction))