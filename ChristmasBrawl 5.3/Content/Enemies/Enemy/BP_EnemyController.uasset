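; AI controller for an enemy that runs the BT_EnemyBehavior behavior tree when play begins.
; PawnSensing sight writes any seen VRPawn to the blackboard as the player.
; An UpdateSoundBB helper stores a sound's location and a heard flag, but its distance-checked call is disconnected from the empty OnHearNoise event, so hearing is inactive.
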(event OnSeePawn(PawnSensing)
  (params (Pawn :type Pawn%20Object%20Reference))
  (bind _asvrpawn (Utilities|Casting|CastToVRPawn Pawn))
  (AI|Components|Blackboard|SetValueasObject (AI|GetBlackboard 0) (Variables|Default|GetPlayerKeyName) _asvrpawn))

(event OnHearNoise(PawnSensing)
  (params (Instigator :type Pawn%20Object%20Reference) (Location :type Vector%20%28by%20ref%29 :default "0, 0, 0") (Volume :type Float%20%28single-precision%29)))

(event EventBeginPlay
  (AI|RunBehaviorTree "/Game/Enemies/Enemy/BT_EnemyBehavior.BT_EnemyBehavior"))

(event EventTick
  (params (DeltaSeconds :type Float%20%28single-precision%29)))

(fn ConstructionScript)